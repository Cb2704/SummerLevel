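; BP_Player is the player character, delegating its movement logic to the BPPlayerMovement component.
; The construction script seeds that component with the camera's relative transform, capsule half height and player options, while landing and capsule hit events are forwarded to it at runtime.
; BeginPlay adds the main screen widget to the player's screen.
; AnyDamage subtracts from Health and only prints debug text, including "Game Over" at zero or below.
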(event OnComponentHit(CapsuleComponent)
  (params (HitComponent :type Primitive%20Component%20Object%20Reference) (OtherActor :type Actor%20Object%20Reference) (OtherComp :type Primitive%20Component%20Object%20Reference) (NormalImpulse :type Vector :default "0, 0, 0") (Hit :type Hit%20Result%20Structure%20%28by%20ref%29))
  ;[0.0706 0 0.125] Capsule Hit
  (Class|BPIPlayer|PlayerCapsuleComponentHit(Message) (Variables|Default|GetBP_PlayerMovement) Hit))

(event EventOnLanded
  (params (Hit :type Hit%20Result%20Structure%20%28by%20ref%29))
  ;[0.0706 0 0.125] On Landed
  (Class|BPIPlayer|PlayeronLanded(Message) (Variables|Default|GetBP_PlayerMovement) Hit))

(event EventBeginPlay
  ;[0.0706 0 0.125] Begin Play
  (bind _returnvalue (UserInterface|CreateWidget "/Game/FastMovement/Widgets/WBP_Main_Screen.WBP_Main_Screen_C"))
  (UserInterface|Viewport|AddtoPlayerScreen _returnvalue))

(event Game|Damage|EventAnyDamage
  (params (Damage :type Float%20%28single-precision%29) (DamageType :type Damage%20Type%20Object%20Reference) (InstigatedBy :type Controller%20Object%20Reference) (DamageCauser :type Actor%20Object%20Reference))
  (Variables|Default|SetHealth (- (Variables|Default|GetHealth) Damage))
  (Development|PrintString "Hello")
  (if (<= (Variables|Default|GetHealth) 0.0)
    (Development|PrintString "Game Over")))

(fn ConstructionScript
  (bind _bp_playermovement (Variables|Default|GetBP_PlayerMovement))
  ;[0.1519 0.1561 0.2917] Event Construct
  (Variables|/Game/FastMovement/Blueprints/Player/BP_PlayerMovement.BP_PlayerMovement_C|SetPlayerCameraRelativeTransorm _bp_playermovement (Transformation|GetRelativeTransform (Variables|Default|GetCamera)))
  (Variables|/Game/FastMovement/Blueprints/Player/BP_PlayerMovement.BP_PlayerMovement_C|SetPlayerCapsuleHalfHeight _bp_playermovement (Variables|/Script/Engine.CapsuleComponent|GetCapsuleHalfHeight (Variables|Collision|GetCapsuleComponent)))
  (Variables|/Game/FastMovement/Blueprints/Player/BP_PlayerMovement.BP_PlayerMovement_C|SetStruct%20Player%20Options _bp_playermovement (Variables|Default|GetPlayerOptions)))