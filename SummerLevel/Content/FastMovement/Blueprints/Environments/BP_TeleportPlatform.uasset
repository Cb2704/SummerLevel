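; BP_TeleportPlatform is a platform that teleports the player to an assigned TargetPoint when the player hits its cube.
; The hit plays a camera shake, moves BP_Player to the target, then sets control yaw from the target or player rotation, depending on UseActorDirection.
; The construction script draws a brief debug line from the platform to its target to show the link.
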(event OnComponentHit(Cube)
  (params (HitComponent :type Primitive%20Component%20Object%20Reference) (OtherActor :type Actor%20Object%20Reference) (OtherComp :type Primitive%20Component%20Object%20Reference) (NormalImpulse :type Vector :default "0, 0, 0") (Hit :type Hit%20Result%20Structure%20%28by%20ref%29))
  (bind _returnvalue (Game|GetPlayerController 0))
  (bind _targetpoint (Variables|Default|GetTargetPoint))
  (bind _returnvalue_2 (Pawn|GetControlRotation _returnvalue :!class /Script/Engine.Controller))
  ;[0.0706 0 0.125] Component Hit
  (Utilities|IsValid _targetpoint
    (:Is%20Valid
      (if (== OtherActor (Game|Player|GetPlayerPawn 0))
        (bind _asbp_player (Utilities|Casting|CastToBP_Player OtherActor))
        (Game|Feedback|ClientStartCameraShake _returnvalue "/Game/FastMovement/Blueprints/Player/CameraShake/CS_Teleport.CS_Teleport_C" 1.0 "CameraLocal" "0, 0, 0")
        (Transformation|Teleport _asbp_player (Transformation|GetWorldLocation (Variables|/Script/Engine.Actor|GetRootComponent _targetpoint)) "0, 0, 0")
        (Pawn|SetControlRotation _returnvalue (Math|Rotator|MakeRotator (.roll _returnvalue_2) (.pitch _returnvalue_2) (.Yaw (Math|Rotator|BreakRotator (select (Variables|Default|GetUseActorDirection) (Transformation|GetWorldRotation (Variables|/Script/Engine.Actor|GetRootComponent _targetpoint)) (Transformation|GetActorRotation _asbp_player))))))))))

(fn ConstructionScript
  (Rendering|Debug|DrawDebugLine (Transformation|GetActorLocation) (Transformation|GetActorLocation (Variables|Default|GetTargetPoint)) "(R=1.000000,G=0.000000,B=0.834170,A=1.000000)" 1.0 1e+01))