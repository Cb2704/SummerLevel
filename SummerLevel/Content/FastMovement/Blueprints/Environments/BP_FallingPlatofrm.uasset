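; BP_FallingPlatofrm is a platform that temporarily gives way after the player pawn hits its Cube component.
; After a delay, it disables the cube's collision and applies a faded dynamic instance of MI_Solid_Cyan, without moving the cube.
; A second delay restores full opacity and query-only collision, then resets the DoOnce gate that blocks repeat triggers during the cycle.
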(event OnComponentHit(Cube)
  (params (HitComponent :type Primitive%20Component%20Object%20Reference) (OtherActor :type Actor%20Object%20Reference) (OtherComp :type Primitive%20Component%20Object%20Reference) (NormalImpulse :type Vector :default "0, 0, 0") (Hit :type Hit%20Result%20Structure%20%28by%20ref%29))
  ;[0.0706 0 0.125] Component Hit
  (if (== OtherActor (Game|Player|GetPlayerPawn 0))
    (Utilities|FlowControl|DoOnce false :!label _label
      (:Completed
        (Utilities|FlowControl|Delay (Variables|Default|GetDisableCollisionDuration))
        (Collision|SetCollisionEnabled (Variables|Default|GetCube) "NoCollision")
        (bind _returnvalue (Rendering|Material|CreateDynamicMaterialInstance (Variables|Default|GetCube) 0 "/Game/FastMovement/Demo/LevelPrototyping/Materials/MI_Solid_Cyan.MI_Solid_Cyan" "None" :!class /Script/Engine.PrimitiveComponent))
        (Rendering|Material|SetScalarParameterValue _returnvalue "Opacity" 0.2 :!class /Script/Engine.MaterialInstanceDynamic)
        (Utilities|FlowControl|Delay (Variables|Default|GetResetCollisionDuration))
        (Collision|SetCollisionEnabled (Variables|Default|GetCube) "QueryOnly")
        (Rendering|Material|SetScalarParameterValue _returnvalue "Opacity" 1.0 :!class /Script/Engine.MaterialInstanceDynamic)
        (goto _label Reset)))))

(fn ConstructionScript)