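; BP_ShootingEnemy is an enemy that turns toward the player and shoots when its PawnSensing component sees a BP_Player.
; Each sighting spawns an actor at SpawnProjectileLocation and immediately applies damage to the player, independent of any hit.
; It then clears CanAttack and restores it after a short delay, though this graph never checks that flag before firing.
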(event OnSeePawn(PawnSensing)
  (params (Pawn :type Pawn%20Object%20Reference))
  (bind _asbp_player (Utilities|Casting|CastToBP_Player Pawn))
  (Transformation|SetActorRotation (Math|Rotator|FindLookatRotation (Transformation|GetActorLocation) (Transformation|GetActorLocation _asbp_player)))
  (Game|SpawnActorfromClass 0 (Transformation|GetWorldTransform (Variables|Default|GetSpawnProjectileLocation)) "Undefined" "MultiplyWithRoot" 0)
  (Game|Damage|ApplyDamage _asbp_player 1.0 0 0)
  (Variables|Default|SetCanAttack? false)
  (Utilities|FlowControl|Delay 0.4)
  (Variables|Default|SetCanAttack? true))

(event EventBeginPlay)

(event Collision|EventActorBeginOverlap
  (params (OtherActor :type Actor%20Object%20Reference)))

(event EventTick
  (params (DeltaSeconds :type Float%20%28single-precision%29)))

(fn ConstructionScript)