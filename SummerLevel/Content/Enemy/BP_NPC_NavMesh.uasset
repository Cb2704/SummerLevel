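; BP_NPC_NavMesh is an enemy NPC that wanders the navmesh and chases the player when it sees them.
; PawnSensing stores a seen BP_Player and sets SeeingPlayer, which a retriggerable delay clears shortly after sightings stop.
; Tick uses that flag to either re-issue AI MoveTo toward the player's location or start timed moves to random reachable nearby points, with DoOnce nodes gating both branches.
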(event OnSeePawn(PawnSensing)
  (params (Pawn :type Pawn%20Object%20Reference))
  (bind _asbp_player (Utilities|Casting|CastToBP_Player Pawn))
  (Variables|Default|SetPlayer%20Follow _asbp_player)
  (Utilities|FlowControl|Sequence
    (:then_0
      (Variables|Default|SetSeeingPlayer true))
    (:then_1
      (Utilities|FlowControl|RetriggerableDelay 0.6)
      (Variables|Default|SetSeeingPlayer false))))

(event Custom|MoveNPC
  (bind _output_get (Variables|Default|SetRandom%20Location (.RandomLocation (AI|Navigation|GetRandomReachablePointinRadius (Transformation|GetActorLocation) 1e+03 0 0))))
  (AI|AIMoveTo self _output_get 0 5.0 false))

(event EventTick
  (params (DeltaSeconds :type Float%20%28single-precision%29))
  (if (Variables|Default|GetSeeingPlayer)
    (Utilities|FlowControl|DoOnce false :!label _label
      (:Completed
        (AI|AIMoveTo self (Transformation|GetActorLocation (Variables|Default|GetPlayer%20Follow)) 0 5.0 false
          (:then
            (goto _label Reset)))))
    (else
      (Utilities|FlowControl|DoOnce false :!label _label_2
        (:Completed
          (CallFunction|MoveNPC)
          (Utilities|FlowControl|Delay 3.0)
          (goto _label_2 Reset))))))

(fn ConstructionScript)